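; Character Blueprint with a cube mesh whose body color shows whether the character is active.
; The construction script creates a dynamic material instance from the cube's first material and stores it as PlayerMat.
; The ChangeCharacter event checks GetIsActive and sets the BodyColor parameter to a saturated green when active or a paler green when inactive.
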(event EventChangeCharacter
  (bind _playermat (Variables|Default|GetPlayerMat))
  (bind _returnvalue (Class|CharacterCube|GetIsActive))
  (if _returnvalue
    (Rendering|Material|SetVectorParameterValue _playermat "BodyColor" "(R=0.222582,G=1.000000,B=0.000000,A=1.000000)" :!class /Script/Engine.MaterialInstanceDynamic)
    (else
      (Rendering|Material|SetVectorParameterValue _playermat "BodyColor" "(R=0.489575,G=1.000000,B=0.411458,A=1.000000)" :!class /Script/Engine.MaterialInstanceDynamic))))

(fn ConstructionScript
  (bind _cube (Variables|Default|GetCube))
  (bind _returnvalue (Rendering|Material|CreateDynamicMaterialInstance _cube 0 (Utilities|Array|Get(acopy) (Rendering|Material|GetMaterials _cube)) "None" :!class /Script/Engine.PrimitiveComponent))
  (Variables|Default|SetPlayerMat _returnvalue))