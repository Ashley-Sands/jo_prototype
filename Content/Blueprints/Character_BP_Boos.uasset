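; Boos character Blueprint that shows whether it is active through the body color of its Cube mesh.
; The construction script creates a dynamic material instance on the Cube's first material slot and stores it as PlayerMat.
; The ChangeCharacter event checks GetIsActive and sets the BodyColor parameter to saturated red when active, or pale red otherwise.
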(event EventChangeCharacter
  (bind _playermat (Variables|Default|GetPlayerMat))
  (bind _returnvalue (Class|CharacterCube|GetIsActive))
  (if _returnvalue
    (Rendering|Material|SetVectorParameterValue _playermat "BodyColor" "(R=1.000000,G=0.000000,B=0.013262,A=1.000000)" :!class /Script/Engine.MaterialInstanceDynamic)
    (else
      (Rendering|Material|SetVectorParameterValue _playermat "BodyColor" "(R=1.000000,G=0.421875,B=0.428952,A=1.000000)" :!class /Script/Engine.MaterialInstanceDynamic))))

(fn ConstructionScript
  (bind _cube (Variables|Default|GetCube))
  (bind _returnvalue (Rendering|Material|CreateDynamicMaterialInstance _cube 0 (Utilities|Array|Get(acopy) (Rendering|Material|GetMaterials _cube)) "None" :!class /Script/Engine.PrimitiveComponent))
  (Variables|Default|SetPlayerMat _returnvalue))